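; ScoreActor tracks how many BP_Page actors remain in the level and ends the game when none are left.
; Its Act event creates the ScoreWidget and adds it to the viewport.
; Tick counts pages with GetAllActorsOfClass every frame and writes the count to the score widget.
; At zero it shows a WinnerWidget with the score widget's time, hides the score widget and pauses the game.
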(event Collision|EventActorBeginOverlap
  (params (OtherActor :type Actor%20Object%20Reference)))

(event EventTick
  (params (DeltaSeconds :type Float%20%28single-precision%29))
  (bind _scorewidget (Variables|Default|GetScorewidget))
  (bind _outactors (Actor|GetAllActorsOfClass "/Game/OpenWorld/blueprint/pages/BP_Page.BP_Page_C"))
  (Variables|/Game/OpenWorld/widget/ScoreWidget.ScoreWidget_C|Setcur (Variables|Default|GetScorewidget) (Utilities|Text|ToText(Integer) (Utilities|Array|Length _outactors)))
  (if (== (Utilities|Array|Length _outactors) 0)
    (bind _returnvalue (UserInterface|CreateWidget "/Game/OpenWorld/widget/WinnerWidget.WinnerWidget_C"))
    (UserInterface|Viewport|AddtoViewport _returnvalue 0)
    (Variables|/Game/OpenWorld/widget/WinnerWidget.WinnerWidget_C|Settime _returnvalue (Utilities|Text|ToText(Float) (Variables|/Game/OpenWorld/widget/ScoreWidget.ScoreWidget_C|Gettime _scorewidget) "HalfToEven"))
    (Widget|SetVisibility _scorewidget "Hidden")
    (Game|SetGamePaused true)))

(event EventAct
  (bind _returnvalue (UserInterface|CreateWidget "/Game/OpenWorld/widget/ScoreWidget.ScoreWidget_C"))
  (bind _output_get (Variables|Default|SetScorewidget _returnvalue))
  (UserInterface|Viewport|AddtoViewport _output_get 0))

(fn ConstructionScript)