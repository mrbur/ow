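; BP_Page is an interactable page pickup that shows its text on screen when collected.
; BecomeApply and OutOfApply swap the cube's material between a chosen one and the cached original.
; Interact hides the cube, waits, messages a linked PageActor through an interface, destroys itself, opens W_Page with PageText and clears the player's WhileTaking flag.
; Take hides the cube, updates PageCompassActor's widget array and removes its compass widget.
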(event EventBeginPlay
  (Variables|Default|SetPrevMat (Rendering|Material|GetMaterial (Variables|Default|GetCube) 0)))

(event Collision|EventActorBeginOverlap
  (params (OtherActor :type Actor%20Object%20Reference)))

(event EventTick
  (params (DeltaSeconds :type Float%20%28single-precision%29)))

(event EventBecomeApply
  (Rendering|Material|SetMaterial (Variables|Default|GetCube) 0 (Variables|Default|GetchoosenMath)))

(event EventInteract
  (params (InteractMesh :type Mesh%20Component%20Object%20Reference))
  (Development|SetHiddeninGame (Variables|Default|GetCube) true false)
  (Utilities|FlowControl|Delay 1.0)
  (if (Utilities|DoesObjectImplementInterface (Variables|Default|GetPageActor) "/Game/OpenWorld/blueprint/pages/BPI_PageActorAction.BPI_PageActorAction_C")
    (Class|BPIPageActorAction|Act(Message) (Variables|Default|GetPageActor)))
  (Actor|DestroyActor)
  (bind _returnvalue (UserInterface|CreateWidget "/Game/OpenWorld/widget/W_Page.W_Page_C"))
  (bind _output_get (Variables|Default|SetscreenWidget _returnvalue))
  (UserInterface|Viewport|AddtoViewport _output_get 0)
  (bind _asw_page (Utilities|Casting|CastToW_Page (Variables|Default|GetscreenWidget)))
  (Variables|/Game/OpenWorld/widget/W_Page.W_Page_C|SetviewText _asw_page (Variables|Default|GetPageText))
  (bind _returnvalue_2 (Actor|GetActorOfClass "/Game/OpenWorld/BP_CharacterPlayer.BP_CharacterPlayer_C"))
  (Variables|/Game/OpenWorld/BP_CharacterPlayer.BP_CharacterPlayer_C|SetwhileTaking _returnvalue_2 false))

(event EventOutOfApply
  (Rendering|Material|SetMaterial (Variables|Default|GetCube) 0 (Variables|Default|GetPrevMat)))

(event EventTake
  (Development|SetHiddeninGame (Variables|Default|GetCube) true false)
  (bind _returnvalue (Actor|GetActorOfClass "/Game/OpenWorld/blueprint/pages/PageCompassActor.PageCompassActor_C"))
  (bind _aspage_compass_actor (Utilities|Casting|CastToPageCompassActor _returnvalue))
  (Default|UpdateWidgetArray _aspage_compass_actor (Variables|Default|GetCompasWidgetName))
  (Widget|RemovefromParent (Variables|Default|GetCompasWidget)))

(fn ConstructionScript)