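; Compass manager actor that shows screen markers pointing toward each BP_Page in the level.
; BeginPlay creates a CompassPageWidget per page, storing its world position and name.
; Act adds the widgets to the viewport and starts a fast looping timer that positions them horizontally from the 2D camera-to-page angle, signed by a right-vector dot product.
; UpdateWidgetArray drops a named page's widget from tracking.
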(event Custom|ViewCompass
  (bind _returnvalue (Viewport|GetViewportSize))
  (bind _char (Variables|Default|GetChar))
  (bind _returnvalue_2 (/ (.x _returnvalue) 2.0))
  (bind _camera (Variables|/Game/OpenWorld/BP_CharacterPlayer.BP_CharacterPlayer_C|GetCamera _char))
  (for _array_element (Variables|Default|GetpageCompasWidgetArray)
    (if (Widget|IsVisible _array_element)
      (if (> (Math|Vector2D|DotProduct(2D) (Math|Vector2D|Normalize2D (Math|Conversions|ToVector2D(Vector) (- (Variables|/Game/OpenWorld/widget/CompassPageWidget.CompassPageWidget_C|GetWorldposition _array_element) (Transformation|GetWorldLocation _camera)))) (Math|Conversions|ToVector2D(Vector) (Math|Vector|GetRightVector (Transformation|GetActorRotation _char)))) 0.0)
        (Default|SetPos _array_element (+ _returnvalue_2 (* (Class|KismetMathLibrary|DegAcos (Math|Vector2D|DotProduct(2D) (Math|Vector2D|Normalize2D (Math|Conversions|ToVector2D(Vector) (- (Variables|/Game/OpenWorld/widget/CompassPageWidget.CompassPageWidget_C|GetWorldposition _array_element) (Transformation|GetWorldLocation _camera)))) (Math|Vector2D|Normalize2D (Math|Conversions|ToVector2D(Vector) (Math|Vector|GetForwardVector _camera))))) (Variables|Default|GetViewXCenter))))
        (else
          (Default|SetPos _array_element (- _returnvalue_2 (* (Class|KismetMathLibrary|DegAcos (Math|Vector2D|DotProduct(2D) (Math|Vector2D|Normalize2D (Math|Conversions|ToVector2D(Vector) (- (Variables|/Game/OpenWorld/widget/CompassPageWidget.CompassPageWidget_C|GetWorldposition _array_element) (Transformation|GetWorldLocation _camera)))) (Math|Vector2D|Normalize2D (Math|Conversions|ToVector2D(Vector) (Math|Vector|GetForwardVector _camera))))) (Variables|Default|GetViewXCenter)))))))))

(event Custom|UpdateWidgetArray
  (params (pageName :type String))
  (bind _pagecompaswidgetarray (Variables|Default|GetpageCompasWidgetArray))
  (for _array_element _pagecompaswidgetarray
    (if (Utilities|Enum|Equal(Enum) (Utilities|GetObjectName _array_element) pageName)
      (Utilities|Array|RemoveItem _pagecompaswidgetarray _array_element))))

(event EventBeginPlay
  (bind _outactors (Actor|GetAllActorsOfClass "/Game/OpenWorld/blueprint/pages/BP_Page.BP_Page_C"))
  (bind _output_get (Variables|Default|Setpages _outactors))
  (for _array_element _output_get
    (bind _returnvalue (UserInterface|CreateWidget "/Game/OpenWorld/widget/CompassPageWidget.CompassPageWidget_C"))
    (Variables|/Game/OpenWorld/blueprint/pages/BP_Page.BP_Page_C|SetCompasWidgetName _array_element (Utilities|GetObjectName _returnvalue))
    (bind _output_get_2 (Variables|/Game/OpenWorld/blueprint/pages/BP_Page.BP_Page_C|SetCompasWidget _array_element _returnvalue))
    (Variables|/Game/OpenWorld/widget/CompassPageWidget.CompassPageWidget_C|SetWorldposition _output_get_2 (Transformation|GetWorldLocation (Variables|/Game/OpenWorld/blueprint/pages/BP_Page.BP_Page_C|GetCube _array_element)))
    (Utilities|Array|Add (Variables|Default|GetpageCompasWidgetArray) _output_get_2)
    (Variables|Default|SetViewXCenter (/ (.x (Viewport|GetViewportSize)) 1.8e+02))
    (bind _returnvalue_2 (Actor|GetActorOfClass "/Game/OpenWorld/BP_CharacterPlayer.BP_CharacterPlayer_C"))
    (Variables|Default|SetChar _returnvalue_2)))

(event EventAct
  (Utilities|Time|SetTimerbyEvent (delegate Custom|ViewCompass) 0.01 true)
  (for _array_element (Variables|Default|GetpageCompasWidgetArray)
    (UserInterface|Viewport|AddtoViewport _array_element 0)))

(fn ConstructionScript)

(fn NewFunction0
  (params (color :type Byte) (dest :type Byte))
  (if (== color dest)
    (return color true)
    (elif (< color dest)
      (return (+ color 1) false)
      (else
        (return (- color 1) false)))))