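; Page actor that gradually shifts the level's directional light color to a target DestColor when its Act event is called.
; BeginPlay finds the DirectionalLight and caches its current color as byte RGB.
; Act starts a looping timer after an initial delay; each tick steps every channel one unit toward the target through a helper function and reapplies the color.
; The timer clears once all three channels match.
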(event Custom|CustomEvent_0
  (bind _destcolor (Variables|Default|GetDestColor))
  (bind (_return _newparam) (CallFunction|NewFunction0 (.b (Variables|Default|GetColor)) (.b _destcolor)))
  (bind (_return_2 _newparam_2) (CallFunction|NewFunction0 (.g (Variables|Default|GetColor)) (.g _destcolor)))
  (bind (_return_3 _newparam_3) (CallFunction|NewFunction0 (.r (Variables|Default|GetColor)) (.r _destcolor)))
  (bind _output_get (Variables|Default|SetColor (Math|Color|MakeColor _return _return_2 _return_3 1)))
  (Rendering|Components|Light|SetLightColor (Variables|/Script/Engine.Light|GetLightComponent (Variables|Default|Getdirlight)) (Math|Conversions|ToLinearColor(Color) _output_get) true)
  (if _newparam
    (if _newparam_2
      (if _newparam_3
        (Utilities|Time|ClearandInvalidateTimerbyHandle (stale EventAct _returnvalue))))))

(event EventBeginPlay
  (bind _returnvalue (Actor|GetActorOfClass "/Script/Engine.DirectionalLight"))
  (bind _output_get (Variables|Default|Setdirlight _returnvalue))
  (Variables|Default|SetColor (Math|Conversions|ToColor(LinearColor) (Rendering|Components|Light|GetLightColor (Variables|/Script/Engine.Light|GetLightComponent _output_get)))))

(event Collision|EventActorBeginOverlap
  (params (OtherActor :type Actor%20Object%20Reference)))

(event EventTick
  (params (DeltaSeconds :type Float%20%28single-precision%29)))

(event EventAct
  (bind _returnvalue (Utilities|Time|SetTimerbyEvent (delegate Custom|CustomEvent_0) 0.02 true 3.0)))

(fn ConstructionScript)

(fn NewFunction0
  (params (color :type Byte) (dest :type Byte))
  (if (== color dest)
    (return color true)
    (elif (< color dest)
      (return (+ color 1) false)
      (else
        (return (- color 1) false)))))