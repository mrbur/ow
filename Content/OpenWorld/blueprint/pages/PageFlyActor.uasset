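; PageFlyActor is an actor that switches the player character between flying, physics simulation and walking.
; Act sets the cached character's movement to Flying, while PhysicsOnEvent turns on capsule physics and this actor's Tick.
; Tick sphere-traces just above the player's location; any hit stops physics and ticking and restores Walking.
; An unconnected branch that sets capsule and camera rotations never runs.
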(event Custom|PhysicsOnEvent
  (Physics|SetSimulatePhysics (Variables|/Script/Engine.Character|GetCapsuleComponent (Variables|Default|GetChar)) true)
  (Actor|Tick|SetActorTickEnabled true))

(event Collision|EventActorBeginOverlap
  (params (OtherActor :type Actor%20Object%20Reference)))

(event EventBeginPlay
  (bind _asbp_character_player (Utilities|Casting|CastToBP_CharacterPlayer (Game|Player|GetPlayerPawn 0)))
  (Variables|Default|SetChar _asbp_character_player))

(event EventAct
  (Pawn|Components|CharacterMovement|SetMovementMode (Variables|/Script/Engine.Character|GetCharacterMovement (Variables|Default|GetChar)) "MOVE_Flying" 0))

(event EventTick
  (params (DeltaSeconds :type Float%20%28single-precision%29))
  (bind _returnvalue (Game|Player|GetPlayerPawn 0))
  (bind _char (Variables|Default|GetChar))
  (bind _returnvalue_2 (Transformation|GetActorLocation _returnvalue))
  (bind _outhits (Collision|MultiSphereTraceForObjects _returnvalue_2 (+ _returnvalue_2 "0, 0,100.000000") 1e+02 (Variables|Default|GetObject%20Types) false (Utilities|Array|MakeArray _returnvalue) "None"))
  (if (> (Utilities|Array|Length _outhits) 0)
    (Physics|SetSimulatePhysics (Variables|/Script/Engine.Character|GetCapsuleComponent _char) false)
    (Actor|Tick|SetActorTickEnabled false)
    (Pawn|Components|CharacterMovement|SetMovementMode (Variables|/Script/Engine.Character|GetCharacterMovement _char) "MOVE_Walking" 0)))

(fn ConstructionScript)