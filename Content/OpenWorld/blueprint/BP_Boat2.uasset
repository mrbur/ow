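; BP_Boat2 is an interactable boat actor that hides its Plane and seven Cylinder meshes when play begins.
; Act reveals the cylinders but leaves the Plane hidden.
; Interact calls the empty OutOfApply event and sets IsActing; BecomeApply is also a stub.
; Disconnected nodes for attaching to the interacting mesh's ik_foot_root socket and enabling Plane physics never run.
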(event EventBeginPlay
  (Development|SetHiddeninGame (Variables|Default|GetPlane) true false)
  (Development|SetHiddeninGame (Variables|Default|GetCylinder8) true false)
  (Development|SetHiddeninGame (Variables|Default|GetCylinder7) true false)
  (Development|SetHiddeninGame (Variables|Default|GetCylinder6) true false)
  (Development|SetHiddeninGame (Variables|Default|GetCylinder5) true false)
  (Development|SetHiddeninGame (Variables|Default|GetCylinder4) true false)
  (Development|SetHiddeninGame (Variables|Default|GetCylinder2) true false)
  (Development|SetHiddeninGame (Variables|Default|GetCylinder1) true false))

(event Collision|EventActorBeginOverlap
  (params (OtherActor :type Actor%20Object%20Reference)))

(event EventTick
  (params (DeltaSeconds :type Float%20%28single-precision%29)))

(event EventBecomeApply)

(event EventInteract
  (params (InteractMesh :type Mesh%20Component%20Object%20Reference))
  (CallFunction|OutOfApply)
  (Variables|Default|SetIsActing true))

(event EventOutOfApply)

(event EventAct
  (Development|SetHiddeninGame (Variables|Default|GetCylinder8) false false)
  (Development|SetHiddeninGame (Variables|Default|GetCylinder7) false false)
  (Development|SetHiddeninGame (Variables|Default|GetCylinder6) false false)
  (Development|SetHiddeninGame (Variables|Default|GetCylinder5) false false)
  (Development|SetHiddeninGame (Variables|Default|GetCylinder4) false false)
  (Development|SetHiddeninGame (Variables|Default|GetCylinder2) false false)
  (Development|SetHiddeninGame (Variables|Default|GetCylinder1) false false))

(fn ConstructionScript)