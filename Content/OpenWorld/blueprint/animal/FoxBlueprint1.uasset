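; Fox character Blueprint that the player can control and leave to return to the player character.
; It moves forward every tick along its facing, with input axes for turning, looking and yaw-relative forward movement.
; Any actor overlap switches its movement mode to Flying.
; The BackToBody action makes player controller 0 possess BP_CharacterPlayer and sets that character's movement back to Walking.
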(event EventBeginPlay)

(event Collision|EventActorBeginOverlap
  (params (OtherActor :type Actor%20Object%20Reference))
  (Pawn|Components|CharacterMovement|SetMovementMode (Variables|Character|GetCharacterMovement) "MOVE_Flying" 0))

(event EventTick
  (params (DeltaSeconds :type Float%20%28single-precision%29))
  (Pawn|Input|AddMovementInput (Math|Vector|GetForwardVector (Transformation|GetActorRotation)) 1.0 false))

(event Input|ActionEvents|InputActionBackToBody
  (params (Key :type Key%20Structure :default "None"))
  (:Pressed
    (bind _returnvalue (Actor|GetActorOfClass "/Game/OpenWorld/BP_CharacterPlayer.BP_CharacterPlayer_C"))
    (Pawn|Possess (Game|GetPlayerController 0) _returnvalue)
    (Pawn|Components|CharacterMovement|SetMovementMode (Variables|/Script/Engine.Character|GetCharacterMovement _returnvalue) "MOVE_Walking" 0)))

(event Input|AxisEvents|InputAxisMoveForvard
  (params (AxisValue :type Float%20%28single-precision%29))
  (Pawn|Input|AddMovementInput (Math|Vector|GetForwardVector (Math|Rotator|MakeRotator 0.0 0.0 (.yaw (Pawn|GetControlRotation :!class /Script/Engine.Pawn)))) AxisValue false))

(event Input|AxisEvents|InputAxisLookUp
  (params (AxisValue :type Float%20%28single-precision%29))
  (Pawn|Input|AddControllerPitchInput AxisValue))

(event Input|AxisEvents|InputAxisTurn
  (params (AxisValue :type Float%20%28single-precision%29))
  (Pawn|Input|AddControllerYawInput AxisValue))

(fn ConstructionScript)