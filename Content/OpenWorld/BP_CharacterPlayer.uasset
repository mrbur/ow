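; First-person player character for the open world, with movement, look, jump, pause menu and interaction.
; A box overlap selects the current BPI_Interaction object; taking a BP_Page enables Tick, which pins the camera to a Sphere while FtakePose runs the bend-down.
; The finished pickup saves the page's location as the return point for the possess input and PossEvent.
; Other inputs trigger PageFlyActor physics and trace-enable physics on movable objects.
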(event OnComponentBeginOverlap(Box)
  (params (OverlappedComponent :type Primitive%20Component%20Object%20Reference) (OtherActor :type Actor%20Object%20Reference) (OtherComp :type Primitive%20Component%20Object%20Reference) (OtherBodyIndex :type Integer) (bFromSweep :type Boolean) (SweepResult :type Hit%20Result%20Structure%20%28by%20ref%29))
  (if (Utilities|DoesObjectImplementInterface OtherActor "/Game/OpenWorld/BPI_Interaction.BPI_Interaction_C")
    (Utilities|IsValid (Variables|Default|GetApplyableObj)
      (:Is%20Not%20Valid
        (bind _output_get (Variables|Default|SetApplyableObj OtherActor))
        (Class|BPIInteraction|BecomeApply(Message) _output_get)))))

(event OnComponentEndOverlap(Box)
  (params (OverlappedComponent :type Primitive%20Component%20Object%20Reference) (OtherActor :type Actor%20Object%20Reference) (OtherComp :type Primitive%20Component%20Object%20Reference) (OtherBodyIndex :type Integer))
  (if (Utilities|DoesObjectImplementInterface OtherActor "/Game/OpenWorld/BPI_Interaction.BPI_Interaction_C")
    (if (Variables|Default|GetwhileTaking)
      (Utilities|FlowControl|Delay 3.0))
    (Class|BPIInteraction|OutOfApply(Message) OtherActor)
    (Variables|Default|SetApplyableObj 0)))

(event Custom|Resume
  (bind _returnvalue (Game|GetPlayerController 0))
  (bind _returnvalue_2 (Game|GetPlayerController 0))
  (Utilities|FlowControl|FlipFlop
    (:A
      (Game|SetGamePaused true)
      (bind _returnvalue_3 (UserInterface|CreateWidget "/Game/OpenWorld/widget/W_PauseWidget.W_PauseWidget_C"))
      (bind _output_get (Variables|Default|SetPauseWidget _returnvalue_3))
      (UserInterface|Viewport|AddtoPlayerScreen _output_get)
      (Variables|/Script/Engine.PlayerController|SetbShowMouseCursor _returnvalue true)
      (Input|SetInputModeGameandUI _returnvalue (Variables|Default|GetPauseWidget) "DoNotLock" true))
    (:B
      (Game|SetGamePaused false)
      (Widget|RemovefromParent (Variables|Default|GetPauseWidget))
      (Variables|/Script/Engine.PlayerController|SetbShowMouseCursor _returnvalue_2 false)
      (Input|SetInputModeGameOnly _returnvalue_2))))

(event Custom|PossEvent
  (Transformation|SetWorldLocation (Variables|Default|GetCapsuleComponent) (Variables|Default|GetStartPosition) false false))

(event EventBeginPlay
  (Variables|Default|SetStartPosition (Transformation|GetWorldLocation (Variables|Default|GetCapsuleComponent))))

(event EventTick
  (params (DeltaSeconds :type Float%20%28single-precision%29))
  (bind _applyableobj (Variables|Default|GetApplyableObj))
  (bind _ftake_pose (Variables|Default|Getftake_pose))
  (if (Variables|Default|GetbbendingDown)
    (if (< _ftake_pose 1.0)
      (Class|GameCharacter|SetTakePos (Variables|Default|GetSphere) (Variables|Default|GetCamera) :!label _label)
      (else
        (Variables|Default|SetbbendingDown false)
        (Class|BPIInteraction|Take(Message) _applyableobj)
        (Variables|Default|SetAxis%20Value 0.0)))
    (elif (> _ftake_pose 0.0)
      (goto _label)
      (elif (Variables|Default|GetwhileTaking)
        (Class|BPIInteraction|Interact(Message) _applyableobj (Variables|Character|GetMesh))
        (Transformation|SetRelativeLocation (Variables|Default|GetCamera) "40.000000, 0,60.000000" false false)
        (Variables|Default|SetStartPosition (Transformation|GetActorLocation _applyableobj))
        (Actor|Tick|SetActorTickEnabled false)))))

(event Input|ActionEvents|InputActionpossess
  (params (Key :type Key%20Structure :default "None"))
  (:Pressed
    (Transformation|SetWorldLocation (Variables|Default|GetCapsuleComponent) (Variables|Default|GetStartPosition) false false)))

(event Input|ActionEvents|InputActionTake
  (params (Key :type Key%20Structure :default "None"))
  (bind _applyableobj (Variables|Default|GetApplyableObj))
  (:Released
    (if (Utilities|IsValid (Variables|Default|GetApplyableObj))
      (Utilities|Casting|CastToBP_Page _applyableobj
        (:then
          (Variables|Default|SetbbendingDown true)
          (Variables|Default|SetwhileTaking true)
          (Actor|Tick|SetActorTickEnabled true))
        (:CastFailed
          (Class|BPIInteraction|Interact(Message) _applyableobj (Variables|Character|GetMesh)))))))

(event Input|ActionEvents|InputActionJump
  (params (Key :type Key%20Structure :default "None"))
  (:Pressed
    (Character|Jump)))

(event Input|ActionEvents|InputActionQPause
  (params (Key :type Key%20Structure :default "None"))
  (bind _returnvalue (Game|GetPlayerController 0))
  (bind _returnvalue_2 (Game|GetPlayerController 0))
  (:Pressed
    (Utilities|FlowControl|FlipFlop
      (:A
        (Game|SetGamePaused true)
        (bind _returnvalue_3 (UserInterface|CreateWidget "/Game/OpenWorld/widget/W_PauseWidget.W_PauseWidget_C"))
        (bind _output_get (Variables|Default|SetPauseWidget _returnvalue_3))
        (UserInterface|Viewport|AddtoPlayerScreen _output_get)
        (Variables|/Script/Engine.PlayerController|SetbShowMouseCursor _returnvalue true)
        (Input|SetInputModeGameandUI _returnvalue (Variables|Default|GetPauseWidget) "DoNotLock" true))
      (:B
        (Game|SetGamePaused false)
        (Widget|RemovefromParent (Variables|Default|GetPauseWidget))
        (Variables|/Script/Engine.PlayerController|SetbShowMouseCursor _returnvalue_2 false)
        (Input|SetInputModeGameOnly _returnvalue_2)))))

(event Input|ActionEvents|InputActionStopFly
  (params (Key :type Key%20Structure :default "None"))
  (:Pressed
    (bind _returnvalue (Actor|GetActorOfClass "/Game/OpenWorld/blueprint/pages/PageFlyActor.PageFlyActor_C"))
    (Default|PhysicsonEvent _returnvalue)))

(event Input|ActionEvents|InputActionTraceMovableObj
  (params (Key :type Key%20Structure :default "None"))
  (bind _camera (Variables|Default|GetCamera))
  (bind _returnvalue (Transformation|GetWorldLocation _camera))
  (:Pressed
    (bind _outhit (Collision|LineTraceForObjects _returnvalue (+ _returnvalue (* (Math|Vector|GetForwardVector (Transformation|GetWorldRotation _camera)) 500)) (Variables|Default|GetObject%20Types_0) false 0 "None"))
    (if (Variables|Default|GetCanMoveObj)
      (bind _asbp_movable_obj (Utilities|Casting|CastToBP_MovableObj (.HitActor (Collision|BreakHitResult _outhit))))
      (Physics|SetSimulatePhysics (Variables|/Game/OpenWorld/blueprint/rocks/BP_MovableObj.BP_MovableObj_C|GetStaticMesh _asbp_movable_obj) true))))

(event Input|AxisEvents|InputAxisMoveForvard
  (params (AxisValue :type Float%20%28single-precision%29))
  (if (not (Variables|Default|GetbbendingDown))
    (Pawn|Input|AddMovementInput (Math|Vector|GetForwardVector (Math|Rotator|MakeRotator 0.0 0.0 (.yaw (Pawn|GetControlRotation :!class /Script/Engine.Pawn)))) AxisValue false)))

(event Input|AxisEvents|InputAxisMoveRight
  (params (AxisValue :type Float%20%28single-precision%29))
  (if (not (Variables|Default|GetbbendingDown))
    (Pawn|Input|AddMovementInput (Math|Vector|GetRightVector (Math|Rotator|MakeRotator 0.0 0.0 (.yaw (Pawn|GetControlRotation :!class /Script/Engine.Pawn)))) AxisValue false)))

(event Input|AxisEvents|InputAxisLookUp
  (params (AxisValue :type Float%20%28single-precision%29))
  (if (< (- (Variables|Default|GetAxis%20Value) AxisValue) 8e+01)
    (if (> (- (Variables|Default|GetAxis%20Value) AxisValue) -62.0)
      (Variables|Default|SetAxis%20Value (- (Variables|Default|GetAxis%20Value) AxisValue))
      (CallFunction|SetHeadPosition))))

(event Input|AxisEvents|InputAxisTurn
  (params (AxisValue :type Float%20%28single-precision%29))
  (Pawn|Input|AddControllerYawInput AxisValue))

(fn ConstructionScript)

(fn GetPose
  (return (Variables|Default|Getftake_pose)))

(fn SetTakePosition
  (bind _sphere (Variables|Default|GetSphere))
  (bind _camera (Variables|Default|GetCamera))
  (bind _returnvalue (Transformation|GetWorldRotation _sphere))
  (Transformation|SetWorldRotation _camera (Math|Rotator|MakeRotator (.roll _returnvalue) (.pitch _returnvalue) (.yaw _returnvalue)) true false)
  (Transformation|SetWorldLocation _camera (Transformation|GetWorldLocation _sphere) false false)
  (return))

(fn SetHeadPosition
  (bind _camera (Variables|Default|GetCamera))
  (bind _returnvalue (Transformation|GetWorldRotation _camera))
  (Transformation|SetWorldRotation (Variables|Default|GetCamera) (Math|Rotator|MakeRotator (.roll _returnvalue) (Variables|Default|GetAxis%20Value) (.yaw _returnvalue)) true false)
  (return))